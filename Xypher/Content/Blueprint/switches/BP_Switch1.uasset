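; BP_Switch1 is a lever switch that toggles when Q is pressed, with input enabled while an actor overlaps its Box.
; A FlipFlop alternates between active and inactive, printing the state and calling the EDLeverActive or EDLeverNotActive dispatcher.
; A timeline slides the lever vertically, playing on activation and reversing on deactivation.
; Only activation is gated by a cast of the overlapping actor to BP_ThirdPersonCharacter.
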(event `self.Box.OnComponentBeginOverlap`
  (params (OverlappedComponent :type "PrimitiveComponent Object Reference") (OtherActor :type "Actor Object Reference") (OtherComp :type "PrimitiveComponent Object Reference") (OtherBodyIndex :type Integer) (bFromSweep :type Boolean) (SweepResult :type "HitResult Structure (by ref)"))
  (`self.EnableInput` (`GameplayStatics.GetPlayerController` 0)))

(event `self.Box.OnComponentEndOverlap`
  (params (OverlappedComponent :type "PrimitiveComponent Object Reference") (OtherActor :type "Actor Object Reference") (OtherComp :type "PrimitiveComponent Object Reference") (OtherBodyIndex :type Integer))
  (`self.DisableInput` (`GameplayStatics.GetPlayerController` 0)))

(event `Key|Q`
  (params (Key :type "Key Structure"))
  (:`Pressed`
    (`/Engine/EditorBlueprintResources/StandardMacros.FlipFlop`
      (:`A`
        (`KismetSystemLibrary.PrintString` "Lever is Active" true true (struct :`G` 1.0 :`B` 0.083073 :`A` 1.0))
        (cast `/Game/ThirdPerson/Blueprints/BP_ThirdPersonCharacter` (stale `self.Box.OnComponentBeginOverlap` OtherActor))
        (`self.ED_LeverActive`)
        (bind (_direction _lever_activation_track) (`Timeline|Lever Activation` :!label _label)
          (:`Update`
            (`SceneComponent.K2_SetRelativeLocation` (`self.Lever_`) (`KismetMathLibrary.VLerp` (0.0 0.0 30.0) (0.0 0.0 0.0) _lever_activation_track) false false))))
      (:`B`
        (`KismetSystemLibrary.PrintString` "Lever is Inactive" true true (struct :`R` 1.0 :`B` 0.274688 :`A` 1.0))
        (`self.ED_LeverNotActive`)
        (goto _label :!via `Reverse`)))))

(fn `UserConstructionScript`)