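; BP_Tripwire is a tripwire actor that detects the third-person player character crossing it.
; Its construction script sets the capsule's half height to half the distance between the left and right base components' relative locations, so the trigger length follows their spacing.
; On capsule overlap, it casts the other actor to BP_ThirdPersonCharacter and prints a red message naming it; no other gameplay effect is implemented.
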(event `self.Capsule.OnComponentBeginOverlap`
  (params (OverlappedComponent :type "PrimitiveComponent Object Reference") (OtherActor :type "Actor Object Reference") (OtherComp :type "PrimitiveComponent Object Reference") (OtherBodyIndex :type Integer) (bFromSweep :type Boolean) (SweepResult :type "HitResult Structure (by ref)"))
  (bind _asbp_third_person_character (cast `/Game/ThirdPerson/Blueprints/BP_ThirdPersonCharacter` OtherActor))
  (`KismetSystemLibrary.PrintString` (`KismetStringLibrary.Concat_StrStr` (`KismetSystemLibrary.GetDisplayName` _asbp_third_person_character) "has triggered the tripwire") true true (struct :`R` 1.0 :`B` 0.066405 :`A` 1.0)))

(fn `UserConstructionScript`
  (`CapsuleComponent.SetCapsuleHalfHeight` (`self.Capsule`) (/ (`KismetMathLibrary.Vector_Distance` (`SceneComponent.RelativeLocation` (`self.TripwireBase Left`)) (`SceneComponent.RelativeLocation` (`self.TripwireBase Right`))) 2.0) true))